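; Tank preview actor that displays one of three selectable skins on its body, turret and cannon.
; ApplySkinByIndex maps an index to a skin material, falling back to the first skin for unrecognized values, and stores it as SelectedSkin.
; SetSkins then applies that material to the first material slot of all three components.
; BeginPlay starts the preview with the first skin.
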(event EventBeginPlay
  (Class|TankPreviewActor|ApplySkinbyIndex))

(event EventApplySkinbyIndex
  (params (Index :type Integer))
  (switch int Index
    (:Default
      (Variables|Default|SetSelectedSkin (Variables|Default|GetSkin1) :!label _label))
    (:0
      (goto _label))
    (:1
      (Variables|Default|SetSelectedSkin (Variables|Default|GetSkin2)))
    (:2
      (Variables|Default|SetSelectedSkin (Variables|Default|GetSkin3))))
  (CallFunction|SetSkins))

(fn ConstructionScript)

(fn SetSkins
  (bind _selectedskin (Variables|Default|GetSelectedSkin))
  (Rendering|Material|SetMaterial (Variables|Default|GetBody) 0 _selectedskin)
  (Rendering|Material|SetMaterial (Variables|Default|GetTurret) 0 _selectedskin)
  (Rendering|Material|SetMaterial (Variables|Default|GetCannon) 0 _selectedskin))